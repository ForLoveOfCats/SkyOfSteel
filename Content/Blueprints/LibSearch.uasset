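; LibSearch is a search helper that scores how well an entry matches a search term, ignoring case.
; IsSubword checks whether the term's characters appear in order in the entry, giving MakeScore a base bonus or penalty.
; MakeScore then compares every character pair, rewarding matches, start positions and following-character runs, and penalizing mismatches.
; The run bonuses sit behind NOR-combined length checks, so they only evaluate when both next indices are out of range.
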(fn `Is Subword`
  (params (Entry :type String) (Term :type String))
  (returns (IsSubword :type Boolean))
  (locals (Index :type Integer))
  (bind _returnvalue (`KismetStringLibrary.GetCharacterArrayFromString` Term))
  (bind _index (`local.Index`))
  (for _array_element (`KismetStringLibrary.GetCharacterArrayFromString` Entry)
    (if (`KismetStringLibrary.EqualEqual_StrStr` _array_element (`|GetArrayItem` _returnvalue _index))
      (set `local.Index` (+ _index 1))
      (if (== _index (`KismetArrayLibrary.Array_Length` _returnvalue))
        (return true)))))

(fn `Make Score`
  (params (Entry :type String) (Term :type String))
  (returns (OutScore :type Integer))
  (locals (Score :type Integer))
  (bind _returnvalue (`KismetStringLibrary.ToLower` Entry))
  (bind _returnvalue_2 (`KismetStringLibrary.ToLower` Term))
  (bind _score (`local.Score`))
  (bind _score_2 (`local.Score`))
  (bind _returnvalue_3 (`KismetStringLibrary.GetCharacterArrayFromString` _returnvalue_2))
  (bind _returnvalue_4 (`KismetStringLibrary.GetCharacterArrayFromString` _returnvalue))
  (bind _issubword (`self.Is Subword` _returnvalue _returnvalue_2))
  (if _issubword
    (set `local.Score` (+ _score 15))
    (else
      (set `local.Score` (- _score 5))))
  (for (_array_element _array_index) _returnvalue_4
    (for (_array_element_2 _array_index_2) _returnvalue_3
      (if (`KismetStringLibrary.EqualEqual_StrStr` _array_element_2 _array_element)
        (set `local.Score` (+ _score_2 5))
        (bind _returnvalue_5 (- _array_index 1))
        (if (<= _returnvalue_5 -1)
          (set `local.Score` (+ (`local.Score`) 12) :!label _label)
          (elif (`KismetStringLibrary.EqualEqual_StrStr` (`|GetArrayItem` _returnvalue_4 _returnvalue_5) " ")
            (goto _label)
            (else
              _)))
        (bind _returnvalue_6 (+ _array_index 1))
        (bind _returnvalue_7 (+ _array_index_2 1))
        (if (`KismetMathLibrary.BooleanNOR` (> (`KismetArrayLibrary.Array_Length` _returnvalue_4) _returnvalue_6) (> (`KismetArrayLibrary.Array_Length` _returnvalue_3) _returnvalue_7))
          (if (`KismetStringLibrary.EqualEqual_StrStr` (`|GetArrayItem` _returnvalue_4 _returnvalue_6) (`|GetArrayItem` _returnvalue_3 _returnvalue_7))
            (set `local.Score` (+ (`local.Score`) 10))
            (bind _returnvalue_8 (+ _array_index 2))
            (bind _returnvalue_9 (+ _array_index_2 2))
            (if (`KismetMathLibrary.BooleanNOR` (> (`KismetArrayLibrary.Array_Length` _returnvalue_4) _returnvalue_8) (> (`KismetArrayLibrary.Array_Length` _returnvalue_3) _returnvalue_9))
              (if (`KismetStringLibrary.EqualEqual_StrStr` (`|GetArrayItem` _returnvalue_4 _returnvalue_8) (`|GetArrayItem` _returnvalue_3 _returnvalue_9))
                (set `local.Score` (+ (`local.Score`) 15))))))
        (else
          (`/Engine/EditorBlueprintResources/StandardMacros.DecrementInt` _score_2)))))
  (return (`local.Score`)))