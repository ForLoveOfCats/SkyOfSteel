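; StructureObject is a structure actor that takes its mesh from an item type and animates its scale as it appears.
; On the authority, construction looks up the model by Name and, for one type, sets inventory capacity and seeds an empty inventory with four items.
; BeginPlay runs the BuildScale timeline to scale uniformly when Z scale is not one.
; Give Item and Take Item are unimplemented stubs.
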(event `self.ReceiveBeginPlay`
  (`|ExecutionSequence`
    (:`then_0`
      (if (!= (.z (`self.GetActorScale3D`)) 1.0)
        (bind (_direction _scale) (`Timeline|Build Scale`)
          (:`Update`
            _)
          (:`Finished`
            _))
        (`self.SetActorScale3D` (`KismetMathLibrary.MakeVector` _scale _scale _scale))))
    (:`then_1`
      (if (`self.HasAuthority`)
        _))))

(fn `Give Item`
  (params (Item :type "/Game/Blueprints/InstancedItem Structure"))
  (returns (`Did Succeed` :type Boolean))
  (return false))

(fn `Take Item`
  (params (Name :type "/Game/Blueprints/ItemEnum Enum" :default "NewEnumerator5"))
  (returns (`Found Item` :type Boolean) (Item :type "/Game/Blueprints/InstancedItem Structure")))

(fn `UserConstructionScript`
  (bind _inventory (`self.Inventory`))
  (`/Engine/EditorBlueprintResources/ActorMacros.Switch Has Authority`
    (:`Authority`
      (bind _item_struct (`/Game/Blueprints/ItemLibrary.Return Item Struct` (`self.Name`)))
      (`StaticMeshComponent.SetStaticMesh` (`self.MeshComponent`) (`.Model_15_C3DEF9AF39040C12003100AA44F6C4BD` (break `/Game/Blueprints/ItemInfo` _item_struct)))
      (if (`|EnumEquality` (`self.Name`) "NewEnumerator4")
        (set `self.Max Inventory` 10)
        (if (== (`KismetArrayLibrary.Array_Length` (`self.Inventory`)) 0)
          (`KismetArrayLibrary.Array_Add` _inventory (make `/Game/Blueprints/InstancedItem` "NewEnumerator1"))
          (`KismetArrayLibrary.Array_Add` _inventory (make `/Game/Blueprints/InstancedItem` "NewEnumerator3"))
          (`KismetArrayLibrary.Array_Add` _inventory (make `/Game/Blueprints/InstancedItem` "NewEnumerator0"))
          (`KismetArrayLibrary.Array_Add` _inventory (make `/Game/Blueprints/InstancedItem` "NewEnumerator2")))))))