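; In-game developer console object that runs typed commands for save/load, hosting, connecting, player ID, quitting and display settings.
; RunCommand switches on the first parsed token, calling FirstPersonCharacter for save/load and engine console commands for most others.
; SayOutput and AppendOutput store output and push it to BaseHUD's console widget, with SayOutput also recording history.
; It also binds a create-from-save event that respawns saved StructureObjects with owner and inventory.
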(event `self.ReceiveBeginPlay`
  (`/Engine/EditorBlueprintResources/StandardMacros.DoOnce` false
    (:`Completed`
      (add `self.Create from Save` (delegate `Creating from Save`))
      (`KismetSystemLibrary.PrintString` "Hello"))))

(event `Creating from Save` :!signature `self.Create from Save`
  (params (Structures :type "Array of /Game/Blueprints/SavedStruct Structure (by ref)"))
  (for _array_element Structures
    (bind (_position _rotation _name _ownerusername _inventory) (break `/Game/Blueprints/SavedStruct` _array_element))
    (`|SpawnActorFromClass` "/Game/Blueprints/StructureObject.StructureObject_C" (`KismetMathLibrary.MakeTransform` _position _rotation) "AlwaysSpawn" "OverrideRootScale" null _name _ownerusername _inventory null)))

(fn `AppendOutput`
  (params (Output :type String))
  (`KismetArrayLibrary.Array_Add` (`self.ConsoleOutput`) Output)
  (bind _asbase_hud (cast `/Game/Blueprints/BaseHUD` (`PlayerController.GetHUD` (`GameplayStatics.GetPlayerController` 0))))
  (bind _consolevar (`/Game/Blueprints/BaseHUD.ConsoleVar` _asbase_hud))
  (if (`KismetSystemLibrary.IsValid` _consolevar)
    (`/Game/Blueprints/Console.AddDisplayEntry` _consolevar Output)))

(fn `RunCommand`
  (params (Command :type Text))
  (bind _returnvalue (`KismetTextLibrary.Conv_TextToString` Command))
  (bind _returnvalue_2 (`KismetStringLibrary.ParseIntoArray` _returnvalue))
  (bind _output (`|GetArrayItem` _returnvalue_2 1))
  (bind _output_2 (`|GetArrayItem` _returnvalue_2 1))
  (switch `string` (`|GetArrayItem` _returnvalue_2)
    (:`Default`
      (`self.SayOutput` _returnvalue (`KismetStringLibrary.Concat_StrStr` "Error: \"" _returnvalue "\" is not a valid command.")))
    (:`save`
      (`self.SayOutput` _returnvalue "Attempting to Save.")
      (bind _asfirst_person_character (cast `/Game/Blueprints/FirstPersonCharacter` (`Controller.K2_GetPawn` (`GameplayStatics.GetPlayerController` 0))))
      (`/Game/Blueprints/FirstPersonCharacter.Save Server` _asfirst_person_character))
    (:`load`
      (`self.SayOutput` _returnvalue "Attempting to Load.")
      (bind _asfirst_person_character_2 (cast `/Game/Blueprints/FirstPersonCharacter` (`Controller.K2_GetPawn` (`GameplayStatics.GetPlayerController` 0))))
      (`/Game/Blueprints/FirstPersonCharacter.Load Server` _asfirst_person_character_2))
    (:`get_id`
      (`self.SayOutput` _returnvalue (`KismetStringLibrary.Concat_StrStr` "Your PlayerId is " (`KismetStringLibrary.Conv_IntToString` (`PlayerState.PlayerId` (`Controller.PlayerState` (`self.PlayerController`)))))))
    (:`fps`
      (`self.SayOutput` _returnvalue "Attempting to Toggle FPS Display.")
      (`KismetSystemLibrary.ExecuteConsoleCommand` "stat FPS"))
    (:`quit`
      (`self.SayOutput` _returnvalue "Attempting to Quit.")
      (`KismetSystemLibrary.QuitGame` null "Quit"))
    (:`host`
      (`self.SayOutput` _returnvalue "Attempting to Host.")
      (`KismetSystemLibrary.ExecuteConsoleCommand` "open FirstPersonExampleMap?listen"))
    (:`connect`
      (`self.SayOutput` _returnvalue "Attempting to Connect.")
      (`KismetSystemLibrary.ExecuteConsoleCommand` (`KismetStringLibrary.Concat_StrStr` "open " (`|GetArrayItem` _returnvalue_2 1))))
    (:`gfx_level`
      (`self.SayOutput` _returnvalue "Attempting to Set Graphics Quality Level.")
      (`KismetSystemLibrary.ExecuteConsoleCommand` (`KismetStringLibrary.Concat_StrStr` "sg.PostProcessQuality " (`|GetArrayItem` _returnvalue_2 1))))
    (:`fullscreen`
      (`self.SayOutput` _returnvalue "Attempting to set Fullscreen.")
      (bind _returnvalue_3 (`GameUserSettings.GetGameUserSettings`))
      (switch `string` _output_2
        (:`Default`
          (`self.AppendOutput` (`KismetStringLibrary.Concat_StrStr` "Error: \"" _output_2 "\" is not a Valid Value.")))
        (:`True`
          (bind (_x _y) (break `IntPoint` (`GameUserSettings.GetScreenResolution` _returnvalue_3)))
          (`KismetSystemLibrary.ExecuteConsoleCommand` (`KismetStringLibrary.Concat_StrStr` "r.SetRes " (`KismetStringLibrary.Conv_IntToString` _x) "x" (`KismetStringLibrary.Conv_IntToString` _y) "f")))
        (:`False`
          (`KismetSystemLibrary.ExecuteConsoleCommand` "r.SetRes 800x600w"))))
    (:`shadows`
      (`self.SayOutput` _returnvalue "Attempting to set Shadows Enabled/Disabled.")
      (switch `string` _output
        (:`Default`
          (`self.AppendOutput` (`KismetStringLibrary.Concat_StrStr` "Error: \"" _output "\" is not a Valid Value.")))
        (:`True`
          (`KismetSystemLibrary.ExecuteConsoleCommand` "r.ShadowQuality 3"))
        (:`False`
          (`KismetSystemLibrary.ExecuteConsoleCommand` "r.ShadowQuality 0"))))))

(fn `SayOutput`
  (params (Command :type String) (Output :type String))
  (bind _returnvalue (`KismetStringLibrary.Concat_StrStr` "\n>>> " Command "\n" Output))
  (`KismetArrayLibrary.Array_Add` (`self.ConsoleOutput`) _returnvalue)
  (`KismetArrayLibrary.Array_Add` (`self.ConsoleHistory`) Command)
  (bind _asbase_hud (cast `/Game/Blueprints/BaseHUD` (`PlayerController.GetHUD` (`GameplayStatics.GetPlayerController` 0))))
  (bind _consolevar (`/Game/Blueprints/BaseHUD.ConsoleVar` _asbase_hud))
  (if (`KismetSystemLibrary.IsValid` _consolevar)
    (`/Game/Blueprints/Console.AddDisplayEntry` _consolevar _returnvalue)))

(fn `SetController`
  (params (Controller :type "Controller Object Reference"))
  (set `self.PlayerController` Controller))

(fn `UserConstructionScript`)