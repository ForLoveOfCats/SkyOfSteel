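; ItemLibrary provides a lookup that turns an item name into an item info struct.
; Return Item Struct switches on the name and builds the info from a name and a type enum value.
; All building pieces, such as platforms, walls, slopes, crates and pipes, share one type, while the Error entry has its own.
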(fn `Return Item Struct`
  (params (Name :type "/Game/Blueprints/ItemEnum Enum" :default "NewEnumerator5"))
  (returns (`Item Struct` :type "/Game/Blueprints/ItemInfo Structure"))
  (switch `/Game/Blueprints/ItemEnum` Name
    (:`NewEnumerator5`
      (return (make `/Game/Blueprints/ItemInfo` "NewEnumerator5" "NewEnumerator4" "/Game/Textures/error.error" "/Game/Meshes/error.error" 0 "This object should not exist. If you see this please contact the developer.")))
    (:`NewEnumerator0`
      (return (make `/Game/Blueprints/ItemInfo` "NewEnumerator0" "NewEnumerator0" "/Game/Textures/platform_render.platform_render" "/Game/Meshes/platform.platform" 0 "This object should not exist. If you see this please contact the developer.")))
    (:`NewEnumerator1`
      (return (make `/Game/Blueprints/ItemInfo` "NewEnumerator1" "NewEnumerator0" "/Game/Textures/wall_render.wall_render" "/Game/Meshes/wall.wall" 0 "This object should not exist. If you see this please contact the developer.")))
    (:`NewEnumerator2`
      (return (make `/Game/Blueprints/ItemInfo` "NewEnumerator2" "NewEnumerator0" "/Game/Textures/slope_rendered.slope_rendered" "/Game/Meshes/slope.slope" 0 "This object should not exist. If you see this please contact the developer.")))
    (:`NewEnumerator3`
      (return (make `/Game/Blueprints/ItemInfo` "NewEnumerator3" "NewEnumerator0" "/Game/Textures/slope_down_rendered.slope_down_rendered" "/Game/Meshes/slope_down.slope_down" 0 "This object should not exist. If you see this please contact the developer.")))
    (:`NewEnumerator4`
      (return (make `/Game/Blueprints/ItemInfo` "NewEnumerator4" "NewEnumerator0" "/Game/Textures/error.error" "/Game/Meshes/crate.crate" 0 "This object should not exist. If you see this please contact the developer.")))
    (:`NewEnumerator6`
      (return (make `/Game/Blueprints/ItemInfo` "NewEnumerator6" "NewEnumerator0" "/Game/Textures/error.error" "/Game/Meshes/pipe.pipe" 0 "This object should not exist. If you see this please contact the developer.")))
    (:`NewEnumerator7`
      (return (make `/Game/Blueprints/ItemInfo` "NewEnumerator7" "NewEnumerator0" "/Game/Textures/error.error" "/Game/Meshes/bent_pipe.bent_pipe" 0 "This object should not exist. If you see this please contact the developer.")))))