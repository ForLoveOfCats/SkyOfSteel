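; Function library that saves and loads player-owned structures through a ServerSaveObj save game, returning a status string with the count.
; Save records transform, name, owner and inventory of every StructureObject not owned by "Server" into slot ServerSave.
; Load destroys those non-server structures, then passes the saved array to the first ConsoleObj to recreate them.
; Save's delete targets "Server_Save", unlike the "ServerSave" slot it writes.
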(fn `Load`
  (returns (Log :type String))
  (bind _returnvalue (`GameplayStatics.LoadGameFromSlot` "ServerSave"))
  (bind _asserver_save_obj (cast `/Game/Blueprints/ServerSaveObj` _returnvalue))
  (`|ExecutionSequence`
    (:`then_0`
      (bind _outactors (`GameplayStatics.GetAllActorsOfClass` null "/Game/Blueprints/StructureObject.StructureObject_C"))
      (for _array_element _outactors
        (if (`KismetStringLibrary.NotEqual_StrStr` (`/Game/Blueprints/StructureObject.Owner UserName` _array_element) "Server")
          (`Actor.K2_DestroyActor` _array_element))))
    (:`then_1`
      (bind _outactors_2 (`GameplayStatics.GetAllActorsOfClass` null "/Game/Blueprints/ConsoleObj.ConsoleObj_C"))
      (bind _structureobjects (`/Game/Blueprints/ServerSaveObj.StructureObjects` _asserver_save_obj))
      (`/Game/Blueprints/ConsoleObj.Create from Save` (`|GetArrayItem` _outactors_2) _structureobjects)
      (return (`KismetStringLibrary.Concat_StrStr` "Load Complete.\nFound " (`KismetStringLibrary.Conv_IntToString` (`KismetArrayLibrary.Array_Length` _structureobjects)) " saved structure object.")))))

(fn `Save`
  (returns (Log :type String))
  (locals (StructureObjects :type "Array of /Game/Blueprints/SavedStruct Structure"))
  (bind _structureobjects (`local.StructureObjects`))
  (`GameplayStatics.DeleteGameInSlot` "Server_Save")
  (bind _returnvalue (`GameplayStatics.CreateSaveGameObject` "/Game/Blueprints/ServerSaveObj.ServerSaveObj_C"))
  (bind _outactors (`GameplayStatics.GetAllActorsOfClass` null "/Game/Blueprints/StructureObject.StructureObject_C"))
  (for _array_element _outactors
    (bind _owner_username (`/Game/Blueprints/StructureObject.Owner UserName` _array_element))
    (if (`KismetStringLibrary.NotEqual_StrStr` _owner_username "Server")
      (`KismetArrayLibrary.Array_Add` _structureobjects (make `/Game/Blueprints/SavedStruct` (`Actor.K2_GetActorLocation` _array_element) (`Actor.K2_GetActorRotation` _array_element) (`/Game/Blueprints/StructureObject.Name` _array_element) _owner_username (`/Game/Blueprints/StructureObject.Inventory` _array_element)))))
  (bind _output_get (set `/Game/Blueprints/ServerSaveObj.StructureObjects` _structureobjects _returnvalue))
  (`GameplayStatics.SaveGameToSlot` _returnvalue "ServerSave")
  (return (`KismetStringLibrary.Concat_StrStr` "Save Complete.\nFound " (`KismetStringLibrary.Conv_IntToString` (`KismetArrayLibrary.Array_Length` _output_get)) " savable structure object.")))